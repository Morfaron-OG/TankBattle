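; Player tank Blueprint that hands its barrel and turret components to their reference setters on BeginPlay and handles orbit camera input.
; Horizontal input yaws an azimuth gimbal and vertical input pitches the spring arm, both scaled by frame time.
; Pitch is limited by checking the arm's world rotation and, once out of range, accepting only input back toward it.
; The HorizonRoll action toggles whether the spring arm inherits roll.
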(event EventBeginPlay
  (Class|Tank|SetBarrelReference (Variables|Default|GetTankBarrel))
  (Class|Tank|SetTurretReference (Variables|Default|GetTankTurret)))

(event Input|ActionEvents|InputActionHorizonRoll
  (params (Key :type Key%20Structure :default "AnyKey"))
  (bind _springarm (Variables|Default|GetSpringArm))
  ;[1 1 1] Binding to Change Camera Roll
  (:Pressed
    (if (Variables|/Script/Engine.SpringArmComponent|GetbInheritRoll (Variables|Default|GetSpringArm))
      (Variables|/Script/Engine.SpringArmComponent|SetbInheritRoll _springarm false)
      (else
        (Variables|/Script/Engine.SpringArmComponent|SetbInheritRoll _springarm true)))))

(event Input|AxisEvents|InputAxisCameraRotationHorizontal
  (params (AxisValue :type Float%20%28single-precision%29))
  ;[1 1 1] Horizontal Camera Rotation
  (Transformation|AddLocalRotation (Variables|Default|GetAzimuth%20Gimbal) (Math|Rotator|MakeRotator 0.0 0.0 (* AxisValue (Utilities|Time|GetWorldDeltaSeconds) 1e+02)) false false))

(event Input|AxisEvents|InputAxisCameraRotationVertical
  (params (AxisValue :type Float%20%28single-precision%29))
  (bind _returnvalue (Utilities|Time|GetWorldDeltaSeconds))
  (bind _springarm (Variables|Default|GetSpringArm))
  (bind _returnvalue_2 (Transformation|GetWorldRotation _springarm))
  (bind _returnvalue_3 (* AxisValue _returnvalue 1e+02))
  (bind _returnvalue_4 (>= _returnvalue_3 0.0))
  ;[1 1 1] Camera Pitch Clamped
  (if (<= (.pitch _returnvalue_2) 6.66)
    (if (>= (.pitch _returnvalue_2) -22.5)
      (Transformation|AddLocalRotation _springarm (Math|Rotator|MakeRotator 0.0 _returnvalue_3 0.0) false false :!label _label)
      (elif _returnvalue_4
        (goto _label)))
    (elif (not _returnvalue_4)
      (goto _label))))

(fn ConstructionScript)