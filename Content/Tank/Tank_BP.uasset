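; Tank_BP is a player-controllable tank that wires its aiming, movement, camera and health bar parts together.
; On BeginPlay it passes turret and barrel to TankAiming and both tracks to TankMovement, and gives the HealthBar widget a self reference.
; Input drives an azimuth gimbal and a pitch-clamped spring arm, toggles camera roll inheritance, and forwards fire and movement intents to those components.
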(event EventBeginPlay
  (Class|TankAimingComponent|Initialise (Variables|Default|GetTankAiming) (Variables|Default|GetTurret) (Variables|Default|GetBarrel))
  (Class|TankMovementComponent|Initialise (Variables|Default|GetTankMovement) (Variables|Default|GetLeftTrack) (Variables|Default|GetRightTrack))
  (bind _ashealth_bar (Utilities|Casting|CastToHealthBar (UserInterface|GetUserWidgetObject (Variables|Default|GetWidget))))
  (Variables|/Game/HealthBar.HealthBar_C|SetTankBPRef _ashealth_bar self))

(event Input|ActionEvents|InputActionHorizonRoll
  (params (Key :type Key%20Structure :default "AnyKey"))
  (bind _springarm (Variables|Default|GetSpringArm))
  ;[1 1 1] Binding to Change Camera Roll
  (:Pressed
    (if (Variables|/Script/Engine.SpringArmComponent|GetbInheritRoll (Variables|Default|GetSpringArm))
      (Variables|/Script/Engine.SpringArmComponent|SetbInheritRoll _springarm false)
      (else
        (Variables|/Script/Engine.SpringArmComponent|SetbInheritRoll _springarm true)))))

(event Input|ActionEvents|InputActionFireProjectile
  (params (Key :type Key%20Structure :default "AnyKey"))
  ;[1 1 1] Binding for Firing a Projectile
  (:Pressed
    (Class|TankAimingComponent|FireProjectile (Variables|Default|GetTankAiming))))

(event Input|AxisEvents|InputAxisIntendRotateClockwise
  (params (AxisValue :type Float%20%28single-precision%29))
  ;[1 1 1] Movement Input Binding
  (Class|TankMovementComponent|IntendRotateClockwise (Variables|Default|GetTankMovement) AxisValue))

(event Input|AxisEvents|InputAxisCameraRotationHorizontal
  (params (AxisValue :type Float%20%28single-precision%29))
  ;[1 1 1] Horizontal Camera Rotation
  (Transformation|AddLocalRotation (Variables|Default|GetAzimuth%20Gimbal) (Math|Rotator|MakeRotator 0.0 0.0 (* AxisValue (Utilities|Time|GetWorldDeltaSeconds) 1e+02)) false false))

(event Input|AxisEvents|InputAxisIntendRotateCounterClockwise
  (params (AxisValue :type Float%20%28single-precision%29))
  ;[1 1 1] Movement Input Binding
  (Class|TankMovementComponent|IntendRotateCClockwise (Variables|Default|GetTankMovement) AxisValue))

(event Input|AxisEvents|InputAxisCameraRotationVertical
  (params (AxisValue :type Float%20%28single-precision%29))
  (bind _returnvalue (Utilities|Time|GetWorldDeltaSeconds))
  (bind _springarm (Variables|Default|GetSpringArm))
  (bind _returnvalue_2 (Transformation|GetWorldRotation _springarm))
  (bind _returnvalue_3 (* AxisValue _returnvalue 5e+01))
  (bind _returnvalue_4 (>= _returnvalue_3 0.0))
  ;[1 1 1] Camera Pitch Clamped
  (if (<= (.pitch _returnvalue_2) -5.0)
    (if (>= (.pitch _returnvalue_2) -5e+01)
      (Transformation|AddLocalRotation _springarm (Math|Rotator|MakeRotator 0.0 _returnvalue_3 0.0) false false :!label _label)
      (elif _returnvalue_4
        (goto _label)))
    (elif (not _returnvalue_4)
      (goto _label))))

(event Input|AxisEvents|InputAxisIntendMoveForward
  (params (AxisValue :type Float%20%28single-precision%29))
  ;[1 1 1] Movement Input Binding
  (Class|TankMovementComponent|IntendMoveForwards (Variables|Default|GetTankMovement) AxisValue))

(event Input|AxisEvents|InputAxisIntendMoveBackward
  (params (AxisValue :type Float%20%28single-precision%29))
  ;[1 1 1] Movement Input Binding
  (Class|TankMovementComponent|IntendMoveBackwards (Variables|Default|GetTankMovement) AxisValue))

(fn ConstructionScript)